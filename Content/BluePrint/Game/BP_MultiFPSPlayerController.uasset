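; Player controller for multiplayer FPS deathmatch, linking each player to BP_DeathMatchGameMode for spawning, death, scoring and match updates.
; On death it reports to the game mode, disables input, credits the killer, then destroys the pawn after a delay and requests respawn.
; It spawns and possesses characters on demand, and creates the local HUD, forwarding health, ammo, crosshair recoil and sorted scoreboard updates.
; Client events store the countdown and return to MainMenu at game end.
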(event `ClientDisableInput`
  (`self.DisableInput` (`self.K2_GetPawn`) self))

(event `self.DeathMatch`
  (params (DamageCauser :type "Actor Object Reference"))
  (bind _asbp_death_match_game_mode (cast `/Game/BluePrint/Game/BP_DeathMatchGameMode` (`GameplayStatics.GetGameMode`)))
  (`/Game/BluePrint/Game/BP_DeathMatchGameMode.SelfDeath` _asbp_death_match_game_mode self)
  (`self.ClientDisableInput`)
  (bind _asbp_multi_fpsplayer_controller (cast `/Game/BluePrint/Game/BP_MultiFPSPlayerController` (`self.GetInstigatorController` DamageCauser))
    (:`then`
      (`/Game/BluePrint/Game/BP_DeathMatchGameMode.KillAnother` _asbp_death_match_game_mode _asbp_multi_fpsplayer_controller 15))
    (:`CastFailed`
      _))
  (`KismetSystemLibrary.Delay` 1.0)
  (`self.K2_DestroyActor` (`self.K2_GetPawn`))
  (bind _asbp_death_match_game_mode_2 (cast `/Game/BluePrint/Game/BP_DeathMatchGameMode` (`GameplayStatics.GetGameMode`)))
  (`/Game/BluePrint/Game/BP_DeathMatchGameMode.RequestSpawn` _asbp_death_match_game_mode_2 self))

(event `ServerRequireUpdate`
  (bind _asbp_death_match_game_mode (cast `/Game/BluePrint/Game/BP_DeathMatchGameMode` (`GameplayStatics.GetGameMode`)))
  (`/Game/BluePrint/Game/BP_DeathMatchGameMode.UpdateValue` _asbp_death_match_game_mode))

(event `UpdateValues`
  (params (Valus :type "Array of DeathMatchPlayerData Structure"))
  (bind _output_get (set `self.Valus` Valus))
  (`KisMetMultiFPSLibrary.SortValues` _output_get)
  (bind _playerui (`self.PlayerUI`)
    (:`then`
      (`/Game/BluePrint/GameUI/W_PlayerUI.UpdateSortBox` _playerui (`self.Valus`)))
    (:`else`)))

(event `ClientUpdateDownTime`
  (params (DownTime :type Integer))
  (set `self.DownTime` DownTime))

(event `ClientEndGame`
  (`GameplayStatics.OpenLevel` "MainMenu"))

(event `ClientHideMouse`
  (`WidgetBlueprintLibrary.SetInputMode_GameOnly` self)
  (set `self.bShowMouseCursor` false))

(event `SpawnPlayerCharacter`
  (params (Class :type "HomeworkCharacter Class Reference") (SpawnTransform :type "Transform Structure"))
  (bind _returnvalue (`|SpawnActorFromClass` Class SpawnTransform "Undefined" "OverrideRootScale" null null))
  (`self.Possess` _returnvalue))

(event `StartSpawnCharacter`
  (`KismetSystemLibrary.Delay` 1.0)
  (bind _asbp_death_match_game_mode (cast `/Game/BluePrint/Game/BP_DeathMatchGameMode` (`GameplayStatics.GetGameMode`)))
  (`/Game/BluePrint/Game/BP_DeathMatchGameMode.RequestSpawn` _asbp_death_match_game_mode self))

(event `self.CreatPlayerUI`
  ;[1 1 1] UI
  (`self.PlayerUI`
    (:`then`
      (`Widget.RemoveFromParent` (`self.PlayerUI`)))
    (:`else`
      _))
  (if (`self.IsLocalPlayerController`)
    (bind _returnvalue (`|CreateWidget` "/Game/BluePrint/GameUI/W_PlayerUI.W_PlayerUI_C" self))
    (bind _output_get (set `self.PlayerUI` _returnvalue))
    (`UserWidget.AddToViewport` _output_get 0)
    (`self.ServerRequireUpdate`)))

(event `self.DoCrosshairRecoil`
  ;[1 1 1] UI
  (`/Game/BluePrint/GameUI/W_PlayerUI.DoCrosshairRecoil` (`self.PlayerUI`)))

(event `self.UpdateHPUI`
  (params (CurrHP :type Integer) (Percent :type "Float (single-precision)"))
  ;[1 1 1] UI
  (`/Game/BluePrint/GameUI/W_PlayerUI.UpdateHP` (`self.PlayerUI`) Percent CurrHP))

(event `self.UpdateBulletUI`
  (params (ClipCurrBullet :type Integer) (GunCurrBullet :type Integer))
  ;[1 1 1] UI
  (`/Game/BluePrint/GameUI/W_PlayerUI.UpdateBullet` (`self.PlayerUI`) ClipCurrBullet GunCurrBullet))

(fn `UserConstructionScript`)