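; Deathmatch game mode for a multiplayer FPS that runs the round timer, spawning and per-player scoring.
; The first login becomes session owner and starts a one-second countdown pushed to every client.
; Spawn requests cycle through PlayerStarts, while deaths and kills update a controller-keyed score map broadcast to all players.
; At time zero, other clients end first, then the session is destroyed before the owner ends.
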(event `GameStateSet`
  (bind _outactors (`GameplayStatics.GetAllActorsOfClass` "/Script/Engine.PlayerStart"))
  (set `self.CharacterPoints` _outactors)
  (bind _returnvalue (`KismetSystemLibrary.K2_SetTimerDelegate` (delegate `Down`) 1.0 true))
  (set `self.DownTimeHandle` _returnvalue))

(event `EndGame`
  (bind _ssessionowner (`self.SsessionOwner`))
  (bind _keys (`BlueprintMapLibrary.Map_Keys` (`self.PlayerScoreMap`)))
  (for _array_element _keys
    (if (not (== _array_element _ssessionowner))
      (`/Game/BluePrint/Game/BP_MultiFPSPlayerController.ClientEndGame` _array_element)))
  (`DestroySessionCallbackProxy.DestroySession` _ssessionowner
    (:`then`
      (`/Game/BluePrint/Game/BP_MultiFPSPlayerController.ClientEndGame` _ssessionowner))))

(event `Down`
  (set `self.RoundTime` (- (`self.RoundTime`) 1))
  (bind _keys (`BlueprintMapLibrary.Map_Keys` (`self.PlayerScoreMap`)))
  (for _array_element _keys
    (`/Game/BluePrint/Game/BP_MultiFPSPlayerController.ClientUpdateDownTime` _array_element (`self.RoundTime`)))
  (if (<= (`self.RoundTime`) 0)
    (`KismetSystemLibrary.K2_ClearAndInvalidateTimerHandle` (`self.DownTimeHandle`))
    (`self.EndGame`)))

(event `self.K2_PostLogin`
  (params (NewPlayer :type "PlayerController Object Reference"))
  ;[1 1 1] Login
  (bind _asbp_multi_fpsplayer_controller (cast `/Game/BluePrint/Game/BP_MultiFPSPlayerController` NewPlayer))
  (if (not (`self.FirstJoin`))
    (`self.GameStateSet`)
    (set `self.SsessionOwner` _asbp_multi_fpsplayer_controller)
    (set `self.FirstJoin` true))
  (`/Game/BluePrint/Game/BP_MultiFPSPlayerController.StartSpawnCharacter` _asbp_multi_fpsplayer_controller)
  (`BlueprintMapLibrary.Map_Add` (`self.PlayerScoreMap`) _asbp_multi_fpsplayer_controller (make `DeathMatchPlayerData` (`KismetStringLibrary.Conv_StringToName` (`KismetSystemLibrary.GetObjectName` _asbp_multi_fpsplayer_controller)))))

(event `RequestSpawn`
  (params (PlayerController :type "/Game/BluePrint/Game/BP_MultiFPSPlayerController Object Reference"))
  (bind _spawnindex (`self.SpawnIndex`))
  ;[1 1 1] SpawnPlayer
  (`/Game/BluePrint/Game/BP_MultiFPSPlayerController.SpawnPlayerCharacter` PlayerController "/Game/BluePrint/player/BP_Attack.BP_Attack_C" (`self.GetTransform` (`|GetArrayItem` (`self.CharacterPoints`) (`self.SpawnIndex`))))
  (set `self.SpawnIndex` (+ _spawnindex 1))
  (if (>= _spawnindex (`KismetArrayLibrary.Array_Length` (`self.CharacterPoints`)))
    (set `self.SpawnIndex` 0)))

(event `UpdateValue`
  (bind _playerscoremap (`self.PlayerScoreMap`))
  (bind _keys (`BlueprintMapLibrary.Map_Keys` _playerscoremap))
  (for _array_element _keys
    (bind _values (`BlueprintMapLibrary.Map_Values` _playerscoremap))
    (`/Game/BluePrint/Game/BP_MultiFPSPlayerController.UpdateValues` _array_element _values)))

(event `SelfDeath`
  (params (PlyerController :type "/Game/BluePrint/Game/BP_MultiFPSPlayerController Object Reference"))
  (bind _playerscoremap (`self.PlayerScoreMap`))
  (bind (_value _returnvalue) (`BlueprintMapLibrary.Map_Find` (`self.PlayerScoreMap`) PlyerController))
  (bind (_playername _playerscore) (break `DeathMatchPlayerData` _value))
  ;[1 1 1] 重生数据处理
  (if _returnvalue
    (set `self.TempName` _playername)
    (if (>= _playerscore 10)
      (set `self. TempScore` (- _playerscore 10))
      (else
        (set `self. TempScore` 0)))
    (`BlueprintMapLibrary.Map_Remove` _playerscoremap PlyerController)
    (`BlueprintMapLibrary.Map_Add` _playerscoremap PlyerController (make `DeathMatchPlayerData` (`self.TempName`) (`self. TempScore`)))
    (`self.UpdateValue`)))

(event `KillAnother`
  (params (PlayerController :type "/Game/BluePrint/Game/BP_MultiFPSPlayerController Object Reference") (GetScore :type Integer))
  (bind _playerscoremap (`self.PlayerScoreMap`))
  (bind (_playername _playerscore) (break `DeathMatchPlayerData` (`BlueprintMapLibrary.Map_Find` (`self.PlayerScoreMap`) PlayerController)))
  ;[1 1 1] 重生数据处理
  (set `self.KillTempName` _playername)
  (set `self.KillTempScore` (+ _playerscore GetScore))
  (`BlueprintMapLibrary.Map_Remove` _playerscoremap PlayerController)
  (`BlueprintMapLibrary.Map_Add` _playerscoremap PlayerController (make `DeathMatchPlayerData` (`self.KillTempName`) (`self.KillTempScore`)))
  (`self.UpdateValue`))

(fn `UserConstructionScript`)