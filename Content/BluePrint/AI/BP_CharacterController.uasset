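; AI controller for deathmatch enemies that handles spawning, possession and a perception-triggered attack on the player character.
; SpawnAI creates and possesses a BP_Enemy, cycling through the game mode's CharacterPoints; its looping timer is unconnected.
; On possession it caches the AI character and runs BP_tree if IsSaw, delaying first if IsStart.
; Sensing a HomeworkCharacter clears IsSaw, sets focus, then after a delay fires and applies damage directly through HitedByAI.
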(event `self.ReceiveBeginPlay`)

(event `SpawnAI`
  (bind _spawn_index (`self.Spawn Index`))
  (bind _asbp_death_match_game_mode (cast `/Game/BluePrint/Game/BP_DeathMatchGameMode` (`GameplayStatics.GetGameMode`)))
  (set `self.Character Points` (`/Game/BluePrint/Game/BP_DeathMatchGameMode.CharacterPoints` _asbp_death_match_game_mode))
  (bind _returnvalue (`AIBlueprintHelperLibrary.SpawnAIFromClass` "/Game/BluePrint/AI/BP_Enemy.BP_Enemy_C" null (.location (`self.GetTransform` (`|GetArrayItem` (`self.Character Points`) (`self.Spawn Index`)))) (.rotation (`self.GetTransform` (`|GetArrayItem` (`self.Character Points`) (`self.Spawn Index`)))) false null))
  (`self.Possess` _returnvalue)
  (set `self.Spawn Index` (+ _spawn_index 1))
  (if (>= _spawn_index (`KismetArrayLibrary.Array_Length` (`self.Character Points`)))
    (set `self.Spawn Index` 0)))

(event `self.ReceivePossess`
  (params (PossessedPawn :type "Pawn Object Reference"))
  (bind _asaicharacter (cast `AICharacter` PossessedPawn))
  (set `self.CurAICharacter` _asaicharacter)
  (if (`self.IsStart`)
    (`KismetSystemLibrary.Delay` 5.0)
    (set `self.IsStart` false))
  (if (`self.IsSaw`)
    (`self.RunBehaviorTree` "/Game/BluePrint/AI/BP_tree.BP_tree")))

(event `self.AIPerception.OnTargetPerceptionUpdated`
  (params (Actor :type "Actor Object Reference") (Stimulus :type "AIStimulus Structure"))
  (bind _curaicharacter (`self.CurAICharacter`))
  (bind _ashomework_character (cast `HomeworkCharacter` Actor))
  (if (`.bSuccessfullySensed` (break `AIStimulus` Stimulus))
    (set `self.IsSaw` false)
    (`MagicLeapHMDFunctionLibrary.SetFocusActor` _ashomework_character)
    (`KismetSystemLibrary.Delay` 1.0)
    (`AICharacter.FireWeaponPrimary` _curaicharacter)
    (`HomeworkCharacter.HitedByAI` _ashomework_character _curaicharacter 15.0)))

(fn `UserConstructionScript`)